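; Guard Blueprint that catches the player when something hits its capsule.
; On a capsule hit it plays a quiet siren sound and starts moving the player character toward the StartPosition sprite's world location.
; It then shows the caught-message widget, enables the mouse cursor and pauses the game.
; The hit handler does not check which actor made contact.
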(event OnComponentHit(CapsuleComponent)
  (params (HitComponent :type Primitive%20Component%20Object%20Reference) (OtherActor :type Actor%20Object%20Reference) (OtherComp :type Primitive%20Component%20Object%20Reference) (NormalImpulse :type Vector :default "0, 0, 0") (Hit :type Hit%20Result%20Structure%20%28by%20ref%29))
  ;[1 1 1] Catch player
  (Utilities|FlowControl|Sequence
    (:then_0
      (Audio|PlaySound2D "/Game/sounds/Siren-SoundBible_com-1094437108.Siren-SoundBible_com-1094437108" 0.1 1.0 0.0 0 0))
    (:then_1
      (Components|MoveComponentTo (Variables|/Script/Engine.Actor|GetRootComponent (Game|GetPlayerCharacter 0)) (Transformation|GetWorldLocation (Variables|/Script/Engine.TargetPoint|GetSpriteComponent (Variables|Default|Getstart_position))) "0, 0, 0" false false 0.2 false)
      ;[1 1 1] pop caught message
      (bind _returnvalue (UserInterface|CreateWidget "/Game/Blueprints/youGotCoughtWidget.youGotCoughtWidget_C"))
      (UserInterface|Viewport|AddtoViewport _returnvalue 0)
      (Variables|/Script/Engine.PlayerController|SetbShowMouseCursor (Game|GetPlayerController 0) true)
      (Game|SetGamePaused true))))

(fn ConstructionScript)