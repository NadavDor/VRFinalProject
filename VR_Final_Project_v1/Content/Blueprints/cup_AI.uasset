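; cup_AI is an AI pawn that patrols a route and chases the player in a sneaking game.
; On BeginPlay it moves through four patrol point actors in sequence, pausing briefly at each, then restarts the loop by calling Patrol again.
; When PawnSensing sees a ThirdPersonCharacter, it moves toward that character.
; Reaching the character opens the sneak_out level, while a failed move resumes the patrol.
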(event OnSeePawn(PawnSensing)
  (params (Pawn :type Pawn%20Object%20Reference))
  (bind _asthird_person_character (Utilities|Casting|CastToThirdPersonCharacter Pawn))
  (AI|AIMoveTo self "0, 0, 0" _asthird_person_character 5.0 false
    (:OnSuccess
      (Game|OpenLevel(byName) "sneak_out"))
    (:OnFail
      (CallFunction|Patrol))))

(event Custom|Patrol
  ;[1 1 1] Move in Patrol
  (AI|AIMoveTo self "0, 0, 0" (Variables|Default|GetPatrol1) 5.0 false
    (:OnSuccess
      (Utilities|FlowControl|Delay 2.0)
      (AI|AIMoveTo self "0, 0, 0" (Variables|Default|GetPatrol2) 5.0 false
        (:OnSuccess
          (Utilities|FlowControl|Delay 2.0)
          (AI|AIMoveTo self "0, 0, 0" (Variables|Default|GetPatrol3) 5.0 false
            (:OnSuccess
              (Utilities|FlowControl|Delay 2.0)
              (AI|AIMoveTo self "0, 0, 0" (Variables|Default|GetPatrol4) 5.0 false
                (:OnSuccess
                  (Utilities|FlowControl|Delay 2.0)
                  (CallFunction|Patrol))))))))))

(event EventBeginPlay
  ;[1 1 1] Move in Patrol
  (CallFunction|Patrol))

(fn ConstructionScript)